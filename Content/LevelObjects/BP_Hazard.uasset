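; BP_Hazard is a level volume that either damages or heals third-person characters standing in it, selected by the Healer flag.
; Every Tick it fetches all BP_ThirdPersonCharacter actors and tests each capsule against its Box, polling instead of using overlap events.
; Damage calls LoseHealth only when CanTakeDamage is true, then clears that flag without resetting it here.
; Healing calls GainHealth every frame of overlap, with no gate.
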(event `self.ReceiveTick`
  (params (DeltaSeconds :type "Float (single-precision)"))
  (`|ExecutionSequence`
    (:`then_0`
      (if (not (`self.Healer`))
        (bind _outactors (`GameplayStatics.GetAllActorsOfClass` "/Game/Characters/Player/BP_ThirdPersonCharacter.BP_ThirdPersonCharacter_C"))
        (for _array_element _outactors
          (if (`PrimitiveComponent.IsOverlappingComponent` (`self.Box`) (`Character.CapsuleComponent` _array_element))
            (if (`/Game/Characters/Player/BP_ThirdPersonCharacter.CanTakeDamage` _array_element)
              (set `/Game/Characters/Player/BP_ThirdPersonCharacter.CanTakeDamage` false _array_element)
              (`/Game/Characters/Player/BP_ThirdPersonCharacter.Lose Health` _array_element 10.0))))))
    (:`then_1`
      (if (`self.Healer`)
        (bind _outactors_2 (`GameplayStatics.GetAllActorsOfClass` "/Game/Characters/Player/BP_ThirdPersonCharacter.BP_ThirdPersonCharacter_C"))
        (for _array_element_2 _outactors_2
          (if (`PrimitiveComponent.IsOverlappingComponent` (`self.Box`) (`Character.CapsuleComponent` _array_element_2))
            (`/Game/Characters/Player/BP_ThirdPersonCharacter.Gain Health` _array_element_2 10.0)))))))

(fn `UserConstructionScript`)