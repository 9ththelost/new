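; Harvestable rock that gives resources to the hitting character, with Tiny rocks also collectable into the inventory via Interact.
; BeginPlay optionally randomizes size, which sets health, mesh and yield, with random secondary materials for Medium and Large.
; Each hit subtracts health, adds materials to the player's Items map and pulses the mesh scale.
; At zero health, smaller rocks vanish, while larger ones swap to a Geometry Collection before delayed destruction.
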(event `self.ReceiveBeginPlay`
  (bind _staticmesh (`self.StaticMesh`))
  (bind _staticmesh_2 (`self.StaticMesh`))
  (bind _staticmesh_3 (`self.StaticMesh`))
  (bind _staticmesh_4 (`self.StaticMesh`))
  (if (`self.Randomized`)
    (set `self.Size Number` (`KismetMathLibrary.RandomInteger` 11))
    (if (< (`self.Size Number`) 11)
      (if (< (`self.Size Number`) 9)
        (if (< (`self.Size Number`) 3)
          (if (< (`self.Size Number`) 1)
            (set `self.Size` "NewEnumerator0")
            (else
              (set `self.Size` "NewEnumerator1")))
          (else
            (set `self.Size` "NewEnumerator2")))
        (else
          (set `self.Size` "NewEnumerator3")))
      (if (`|EnumEquality` (`self.Size`) "NewEnumerator0") :!label _label
        (set `self.Health` 0.5)
        (set `self.Material` "NewEnumerator0")
        (set `self.MaterialNum` 1)
        (`StaticMeshComponent.SetStaticMesh` _staticmesh_2 "/Game/DreamscapeSeries/DreamscapeTower/Meshes/Stones/SM_RockSmall_02.SM_RockSmall_02")
        (`PrimitiveComponent.SetCollisionEnabled` _staticmesh_2 "QueryAndPhysics")
        (`SceneComponent.SetVisibility` _staticmesh_2 true false)
        (`SceneComponent.SetRelativeScale3D` _staticmesh_2 (0.5 0.5 0.5))
        (elif (`|EnumEquality` (`self.Size`) "NewEnumerator1")
          (set `self.Health` 2.0)
          (set `self.Material` "NewEnumerator0")
          (set `self.MaterialNum` 1)
          (`StaticMeshComponent.SetStaticMesh` _staticmesh_3 "/Game/DreamscapeSeries/DreamscapeTower/Meshes/Stones/SM_RockSmall_02.SM_RockSmall_02")
          (`PrimitiveComponent.SetCollisionEnabled` _staticmesh_3 "QueryAndPhysics")
          (`SceneComponent.SetVisibility` _staticmesh_3 true false)
          (elif (`|EnumEquality` (`self.Size`) "NewEnumerator2")
            (set `self.Health` 5.0)
            (set `self.Material` "NewEnumerator0")
            (set `self.MaterialNum` 2)
            (set `self.2ndMaterial` (`KismetMathLibrary.RandomInteger` 21))
            (if (< (`self.2ndMaterial`) 9)
              (if (< (`self.2ndMaterial`) 6)
                (if (< (`self.2ndMaterial`) 3)
                  (set `self.Material2` "NewEnumerator2")
                  (else
                    (set `self.Material2` "NewEnumerator1")))
                (else
                  (set `self.Material2` "NewEnumerator0"))))
            (`StaticMeshComponent.SetStaticMesh` _staticmesh_4 "/Game/DreamscapeSeries/DreamscapeTower/Meshes/Stones/SM_RockMedium_01.SM_RockMedium_01")
            (`PrimitiveComponent.SetCollisionEnabled` _staticmesh_4 "QueryAndPhysics")
            (`SceneComponent.SetVisibility` _staticmesh_4 true false)
            (elif (`|EnumEquality` (`self.Size`) "NewEnumerator3")
              (set `self.Health` 10.0)
              (set `self.Material` "NewEnumerator0")
              (set `self.MaterialNum` 2)
              (set `self.2ndMaterial` (`KismetMathLibrary.RandomInteger` 21))
              (if (< (`self.2ndMaterial`) 21)
                (if (< (`self.2ndMaterial`) 12)
                  (if (< (`self.2ndMaterial`) 6)
                    (set `self.Material2` "NewEnumerator2")
                    (else
                      (set `self.Material2` "NewEnumerator1")))
                  (else
                    (set `self.Material2` "NewEnumerator0"))))
              (`StaticMeshComponent.SetStaticMesh` _staticmesh "/Game/DreamscapeSeries/DreamscapeTower/Meshes/Stones/SM_RockMedium_01.SM_RockMedium_01")
              (`PrimitiveComponent.SetCollisionEnabled` _staticmesh "QueryAndPhysics")
              (`SceneComponent.SetVisibility` _staticmesh true false)
              (`SceneComponent.SetRelativeScale3D` _staticmesh (2.0 1.0 1.0)))))))
    (else
      (goto _label))))

(event `self.ReceiveTick`
  (params (DeltaSeconds :type "Float (single-precision)"))
  (bind _smallrock (`self.SmallRock`))
  (bind _output_get (set `self.Chaos Break Event Component` _smallrock))
  (bind _output_get_2 (set `self.Chaos Break Event Location` (`SceneComponent.K2_GetComponentLocation` _smallrock)))
  (bind _output_get_3 (set `self.Chaos Break Event Velocity` (100.0 100.0 100.0)))
  (bind _output_get_4 (set `self.Chaos Break Event Mass` 500.0))
  (`self.Break` _output_get _output_get_2 _output_get_3 (0.0 0.0 0.0) _output_get_4))

(event `Break`
  (params (NewParam :type "PrimitiveComponent Object Reference") (NewParam2 :type "Vector Structure") (NewParam3 :type "Vector Structure") (NewParam4 :type "Vector Structure") (NewParam5 :type "Float (double-precision)")))

(event `/Game/LevelObjects/I_Mine.Hit`
  (params (`Hitting Character` :type "/Game/Characters/Player/BP_ThirdPersonCharacter Object Reference") (Damage :type "Float (double-precision)"))
  ;[0 0.9766 1] event hit
  (`self.NewFunction_0` `Hitting Character` Damage))

(event `destroy tiny`
  ;[0 0.8848 1] destroying
  (`self.K2_DestroyActor` :!label _label_2))

(event `destroy small`
  ;[0 0.8848 1] destroying
  (goto _label_2))

(event `destroy  medium`
  (bind _staticmesh (`self.StaticMesh`))
  (bind (_returnvalue_location _returnvalue_rotation _returnvalue_scale) (`KismetMathLibrary.BreakTransform` (`SceneComponent.GetRelativeTransform` (`self.StaticMesh`))))
  ;[0 0.8848 1] destroying
  (`AddComponent|NODE_AddGeometryCollectionComponent-0` :`RelativeTransform` (`KismetMathLibrary.MakeTransform` (- _returnvalue_location (0.0 0.0 25.0)) _returnvalue_rotation _returnvalue_scale) :!label _label_3)
  (`PrimitiveComponent.SetCollisionEnabled` _staticmesh "NoCollision")
  (`SceneComponent.SetVisibility` _staticmesh false false)
  (`KismetSystemLibrary.Delay` 2.0)
  (`self.K2_DestroyActor`))

(event `self.Interact`
  (params (`Interacting Character` :type "/Game/Characters/Player/BP_ThirdPersonCharacter Object Reference"))
  (bind _ac_iteminfo (`self.AC_ItemInfo`))
  (bind (_currentinfo_name _currentinfo_description _currentinfo_itemclass _currentinfo_icon _currentinfo_mesh _currentinfo_stackable _currentinfo_itemamount) (break `/Game/HUD/Structs/Struct_ItemInfo` (`/Game/HUD/Blueprints/AC_ItemInfo.CurrentInfo` _ac_iteminfo)))
  (if (`|EnumEquality` (`self.Size`) "NewEnumerator0")
    (`/Engine/EditorBlueprintResources/StandardMacros.IsValid` null
      (:`Is Valid`
        (bind _suceeded (`/Game/HUD/Blueprints/AC_Inventory.Add` (`/Game/Characters/Player/BP_ThirdPersonCharacter.AC_Inventory` `Interacting Character`) _currentinfo_name _currentinfo_itemamount (`/Game/HUD/Blueprints/AC_ItemInfo.CurrentInfo` _ac_iteminfo)))
        (if _suceeded
          (`self.K2_DestroyActor`))))))

(event `destroy large`
  ;[0 0.8848 1] destroying
  (goto _label_3))

(event `feedback reaction`
  (bind _staticmesh (`self.StaticMesh`))
  (bind (_returnvalue_x _returnvalue_y _returnvalue_z) (`KismetMathLibrary.BreakVector` (`SceneComponent.K2_GetComponentScale` (`self.StaticMesh`))))
  (bind (_returnvalue_x_2 _returnvalue_y_2 _returnvalue_z_2) (`KismetMathLibrary.BreakVector` (`SceneComponent.K2_GetComponentScale` (`self.StaticMesh`))))
  ;[0 0.8848 1] feedback reaction after hit
  (`/Engine/EditorBlueprintResources/StandardMacros.IsValid` _staticmesh
    (:`Is Valid`
      (`SceneComponent.SetWorldScale3D` _staticmesh (`KismetMathLibrary.MakeVector` (+ _returnvalue_x_2 0.05) (+ _returnvalue_y_2 0.05) (+ _returnvalue_z_2 0.05)))
      (`KismetSystemLibrary.Delay` 0.2)
      (`SceneComponent.SetWorldScale3D` (`self.StaticMesh`) (`KismetMathLibrary.MakeVector` (- _returnvalue_x 0.05) (- _returnvalue_y 0.05) (- _returnvalue_z 0.05))))))

(fn `NewFunction_0`
  (params (player :type "/Game/Characters/Player/BP_ThirdPersonCharacter Object Reference") (damage :type "Float (double-precision)"))
  (locals (`items reference` :type "Map of String to Integer"))
  (bind _health (`self.Health`))
  (bind _returnvalue (/ (`self.MaterialNum`) 2))
  (bind (_value _returnvalue_2) (`BlueprintMapLibrary.Map_Find` (`/Game/Characters/Player/BP_ThirdPersonCharacter.Items` (`local.player`)) (`|GetEnumeratorNameAsString` (`self.Material2`))))
  (bind (_value_2 _returnvalue_3) (`BlueprintMapLibrary.Map_Find` (`/Game/Characters/Player/BP_ThirdPersonCharacter.Items` (`local.player`)) (`|GetEnumeratorNameAsString` (`self.Material`))))
  (set `local.items reference` (`/Game/Characters/Player/BP_ThirdPersonCharacter.Items` player))
  ;[0 0.8848 1] chek if object is already destroyed
  (if (not (<= _health 0.0))
    ;[0 0.8848 1] set object new hp
    (set `self.Health` (- _health (`local.damage`)))
    (`|ExecutionSequence`
      (:`then_0`
        ;[1 0.7969 0] check if the player already is carrying the item in the inventory
        (if _returnvalue_3
          ;[0 0.8848 1] adds the ammount to the inventory slot
          (`BlueprintMapLibrary.Map_Add` (`/Game/Characters/Player/BP_ThirdPersonCharacter.Items` (`local.player`)) (`|GetEnumeratorNameAsString` (`self.Material`)) (+ _value_2 (`self.MaterialNum`)))
          (else
            ;[0 0.8848 1] add the ammount
            (`BlueprintMapLibrary.Map_Add` (`/Game/Characters/Player/BP_ThirdPersonCharacter.Items` (`local.player`)) (`|GetEnumeratorNameAsString` (`self.Material`)) (`self.MaterialNum`))))
        ;[1 0.7302 0] check for another resource
        (if (`|EnumInequality` (`self.Material2`) "NewEnumerator4")
          (if _returnvalue_2
            (`BlueprintMapLibrary.Map_Add` (`/Game/Characters/Player/BP_ThirdPersonCharacter.Items` (`local.player`)) (`|GetEnumeratorNameAsString` (`self.Material2`)) (+ _value _returnvalue))
            (else
              (`BlueprintMapLibrary.Map_Add` (`/Game/Characters/Player/BP_ThirdPersonCharacter.Items` (`local.player`)) (`|GetEnumeratorNameAsString` (`self.Material2`)) _returnvalue))))
        (bind _keys (`BlueprintMapLibrary.Map_Keys` (`/Game/Characters/Player/BP_ThirdPersonCharacter.Items` (`local.player`))))
        (for _array_element _keys
          (`KismetSystemLibrary.PrintString` (`KismetStringLibrary.Concat_StrStr` _array_element ": " (`KismetStringLibrary.Conv_IntToString` (`BlueprintMapLibrary.Map_Find` (`/Game/Characters/Player/BP_ThirdPersonCharacter.Items` (`local.player`)) _array_element))))
          ;[0 0.8848 1] check if item hp is above 0
          (if (<= (`self.Health`) 0.0)
            ;[0 0.8848 1] destroying
            (switch `/Game/Items/Enumerators/E_Size` (`self.Size`)
              (:`NewEnumerator0`
                (`self.destroy tiny`))
              (:`NewEnumerator1`
                (`self.destroy small`))
              (:`NewEnumerator2`
                (`self.destroy  medium`))
              (:`NewEnumerator3`
                (`self.destroy large`))))))
      (:`then_1`
        ;[0 0.8848 1] feedback reaction
        (`self.feedback reaction`)))))

(fn `UserConstructionScript`)