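; BP_Tree is a harvestable bush or tree that gives materials to the character hitting it.
; BeginPlay uses a random or preset Size to set health, yield, meshes and collision.
; Each Hit reduces health, adds materials to the character's Items map and briefly pulses the StaticMesh1 scale.
; At zero health, checked inside the debug key-print loop, Tiny destroys immediately, while larger sizes add a replacement component and destroy after a delay.
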(event `self.ReceiveBeginPlay`
  (bind _staticmesh (`self.StaticMesh`))
  (bind _staticmesh1 (`self.StaticMesh1`))
  (bind _staticmesh1_2 (`self.StaticMesh1`))
  (bind _staticmesh1_3 (`self.StaticMesh1`))
  (bind _staticmesh1_4 (`self.StaticMesh1`))
  (bind _staticmesh_2 (`self.StaticMesh`))
  (if (`self.Randomized`)
    (set `self.Size Number` (`KismetMathLibrary.RandomInteger` 11))
    (if (< (`self.Size Number`) 11)
      (if (< (`self.Size Number`) 9)
        (if (< (`self.Size Number`) 4)
          (if (< (`self.Size Number`) 2)
            (set `self.Size` "NewEnumerator0")
            (else
              (set `self.Size` "NewEnumerator1")))
          (else
            (set `self.Size` "NewEnumerator2")))
        (else
          (set `self.Size` "NewEnumerator3")))
      (`KismetSystemLibrary.PrintString` (`KismetStringLibrary.Conv_IntToString` (`self.Size Number`)))
      (if (`|EnumEquality` (`self.Size`) "NewEnumerator0") :!label _label
        (set `self.Health` 1.0)
        (set `self.Material` "NewEnumerator0")
        (set `self.MaterialNum` 1)
        (`StaticMeshComponent.SetStaticMesh` _staticmesh1 "/Game/DreamscapeSeries/DreamscapeMeadows/Meshes/Foliage/SM_Bushes_New_05.SM_Bushes_New_05")
        (`SceneComponent.SetRelativeScale3D` _staticmesh1 (0.25 0.25 0.25))
        (`PrimitiveComponent.SetCollisionEnabled` _staticmesh1 "QueryAndPhysics")
        (`PrimitiveComponent.SetCollisionEnabled` (`self.Sphere`) "QueryAndPhysics")
        (elif (`|EnumEquality` (`self.Size`) "NewEnumerator1")
          (set `self.Health` 2.0)
          (set `self.Material` "NewEnumerator0")
          (set `self.MaterialNum` 1)
          (`StaticMeshComponent.SetStaticMesh` _staticmesh1_3 "/Game/DreamscapeSeries/DreamscapeMeadows/Meshes/Foliage/SM_Bushes_New_05.SM_Bushes_New_05")
          (`PrimitiveComponent.SetCollisionEnabled` _staticmesh1_3 "QueryAndPhysics")
          (`PrimitiveComponent.SetCollisionEnabled` (`self.Sphere`) "QueryAndPhysics")
          (elif (`|EnumEquality` (`self.Size`) "NewEnumerator2")
            (set `self.Health` 5.0)
            (set `self.Material` "NewEnumerator0")
            (set `self.MaterialNum` 4)
            (set `self.2ndMaterial` (`KismetMathLibrary.RandomInteger` 21))
            (if (< (`self.2ndMaterial`) 8)
              (set `self.Material2` "NewEnumerator0"))
            (`StaticMeshComponent.SetStaticMesh` _staticmesh1_2 "/Game/DreamscapeSeries/DreamscapeMeadows/Meshes/Props/SM_Tree_Stump_01.SM_Tree_Stump_01")
            (`SceneComponent.SetRelativeScale3D` _staticmesh1_2 (0.5 0.5 0.25))
            (`PrimitiveComponent.SetCollisionEnabled` _staticmesh1_2 "QueryAndPhysics")
            (`SceneComponent.SetRelativeScale3D` _staticmesh_2 (1.5 1.5 1.0))
            (`PrimitiveComponent.SetCollisionEnabled` _staticmesh_2 "QueryAndPhysics")
            (`SceneComponent.SetVisibility` _staticmesh_2 true false)
            (elif (`|EnumEquality` (`self.Size`) "NewEnumerator3")
              (set `self.Health` 10.0)
              (set `self.Material` "NewEnumerator0")
              (set `self.MaterialNum` 8)
              (set `self.2ndMaterial` (`KismetMathLibrary.RandomInteger` 21))
              (set `self.Material2` "NewEnumerator0")
              (`StaticMeshComponent.SetStaticMesh` _staticmesh1_4 "/Game/DreamscapeSeries/DreamscapeMeadows/Meshes/Props/SM_Tree_Stump_01.SM_Tree_Stump_01")
              (`SceneComponent.SetRelativeScale3D` _staticmesh1_4 (1.0 1.0 0.5))
              (`PrimitiveComponent.SetCollisionEnabled` _staticmesh1_4 "QueryAndPhysics")
              (`SceneComponent.SetRelativeScale3D` _staticmesh (3.0 3.0 3.5))
              (`PrimitiveComponent.SetCollisionEnabled` _staticmesh "QueryAndPhysics")
              (`SceneComponent.SetVisibility` _staticmesh true false))))))
    (else
      (goto _label))))

(event `/Game/LevelObjects/I_Mine.Hit`
  (params (`Hitting Character` :type "/Game/Characters/Player/BP_ThirdPersonCharacter Object Reference") (Damage :type "Float (double-precision)"))
  (bind _staticmesh (`self.StaticMesh`))
  (bind _health (`self.Health`))
  (bind _staticmesh1 (`self.StaticMesh1`))
  (bind _items (`/Game/Characters/Player/BP_ThirdPersonCharacter.Items` `Hitting Character`))
  (bind _materialnum (`self.MaterialNum`))
  (bind (_returnvalue_location _returnvalue_rotation _returnvalue_scale) (`KismetMathLibrary.BreakTransform` (`SceneComponent.GetRelativeTransform` (`self.StaticMesh`))))
  (bind (_returnvalue_x _returnvalue_y _returnvalue_z) (`KismetMathLibrary.BreakVector` (`SceneComponent.K2_GetComponentScale` (`self.StaticMesh1`))))
  (bind (_returnvalue_x_2 _returnvalue_y_2 _returnvalue_z_2) (`KismetMathLibrary.BreakVector` (`SceneComponent.K2_GetComponentScale` (`self.StaticMesh1`))))
  (bind (_returnvalue_location_2 _returnvalue_rotation_2 _returnvalue_scale_2) (`KismetMathLibrary.BreakTransform` (`SceneComponent.GetRelativeTransform` (`self.StaticMesh1`))))
  (bind _returnvalue (`|GetEnumeratorNameAsString` (`self.Material`)))
  (bind _returnvalue_2 (`|GetEnumeratorNameAsString` (`self.Material2`)))
  (bind _returnvalue_3 (/ (`self.MaterialNum`) 2))
  (bind (_value _returnvalue_4) (`BlueprintMapLibrary.Map_Find` _items _returnvalue_2))
  (bind (_value_2 _returnvalue_5) (`BlueprintMapLibrary.Map_Find` _items _returnvalue))
  (if (not (<= _health 0.0))
    (set `self.Health` (- _health Damage))
    (`|ExecutionSequence`
      (:`then_0`
        (if _returnvalue_5
          (`BlueprintMapLibrary.Map_Add` _items _returnvalue (+ _value_2 _materialnum))
          (else
            (`BlueprintMapLibrary.Map_Add` _items _returnvalue _materialnum)))
        (if (`|EnumInequality` (`self.Material2`) "NewEnumerator1")
          (if _returnvalue_4
            (`BlueprintMapLibrary.Map_Add` _items _returnvalue_2 (+ _value _returnvalue_3))
            (else
              (`BlueprintMapLibrary.Map_Add` _items _returnvalue_2 _returnvalue_3))))
        (bind _keys (`BlueprintMapLibrary.Map_Keys` _items))
        (for _array_element _keys
          (`KismetSystemLibrary.PrintString` (`KismetStringLibrary.Concat_StrStr` _array_element ": " (`KismetStringLibrary.Conv_IntToString` (`BlueprintMapLibrary.Map_Find` _items _array_element))))
          (if (<= (`self.Health`) 0.0)
            (switch `/Game/Items/Enumerators/E_Size` (`self.Size`)
              (:`NewEnumerator0`
                (`self.K2_DestroyActor`))
              (:`NewEnumerator1`
                (`AddComponent|NODE_AddGeometryCollectionComponent-0` :`RelativeTransform` (`KismetMathLibrary.MakeTransform` (- _returnvalue_location_2 (0.0 0.0 25.0)) _returnvalue_rotation_2 _returnvalue_scale_2))
                (`PrimitiveComponent.SetCollisionEnabled` _staticmesh "NoCollision" :!label _label_2)
                (`SceneComponent.SetVisibility` _staticmesh false false)
                (`KismetSystemLibrary.Delay` 2.0)
                (`self.K2_DestroyActor`))
              (:`NewEnumerator2`
                (`AddComponent|NODE_AddStaticMeshComponent-0` :`RelativeTransform` (`KismetMathLibrary.MakeTransform` (+ _returnvalue_location (0.0 0.0 25.0)) _returnvalue_rotation _returnvalue_scale) :!label _label_3)
                (goto _label_2))
              (:`NewEnumerator3`
                (goto _label_3))))))
      (:`then_1`
        (`/Engine/EditorBlueprintResources/StandardMacros.IsValid` _staticmesh1
          (:`Is Valid`
            (`SceneComponent.SetWorldScale3D` _staticmesh1 (`KismetMathLibrary.MakeVector` (+ _returnvalue_x_2 0.05) (+ _returnvalue_y_2 0.05) (+ _returnvalue_z_2 0.05)))
            (`KismetSystemLibrary.Delay` 0.2)
            (`SceneComponent.SetWorldScale3D` (`self.StaticMesh1`) (`KismetMathLibrary.MakeVector` (- _returnvalue_x 0.05) (- _returnvalue_y 0.05) (- _returnvalue_z 0.05)))))))))

(fn `UserConstructionScript`)