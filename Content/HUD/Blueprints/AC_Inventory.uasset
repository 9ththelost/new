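; Inventory actor component that keeps items in a fixed-size Contents array and forwards Server_Interact to the target's AC_ItemInfo with the owning character.
; Add and AddToInventory use FindSlot to increase an existing stack, otherwise CreateStack fills an empty slot.
; FindSlot matches only when the DT_Items stack limit is below zero, and Add mostly passes zero amounts.
; Remove and ChangeSlot are stubs; key 1 prints contents for debugging.
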(event `self.ReceiveBeginPlay`
  (`KismetArrayLibrary.Array_Resize` (`self.Contents`) (`self.MaxSize`)))

(event `InputAction|Main Action`
  (params (Key :type "Key Structure")))

(event `Server_Interact`
  (params (Target :type "Actor Object Reference"))
  (bind _returnvalue (`Actor.GetComponentByClass` Target "/Game/HUD/Blueprints/AC_ItemInfo.AC_ItemInfo_C"))
  (`/Engine/EditorBlueprintResources/StandardMacros.IsValid` _returnvalue
    (:`Is Valid`
      (message `/Game/HUD/Blueprints/I_Interacting.Interact` _returnvalue (cast `/Game/Characters/Player/BP_ThirdPersonCharacter` (`self.GetOwner`) :!pure true)))))

(event `Key|One`
  (params (Key :type "Key Structure"))
  (:`Pressed`
    (`self.DEBUG_PrintContents`)))

(fn `Add`
  (params (`Item Name` :type Name) (`Item Amount` :type Integer) (`Item Info` :type "/Game/HUD/Structs/Struct_ItemInfo Structure"))
  (returns (Suceeded :type Boolean) (Remaining :type Integer))
  (locals (AmountRemaining :type Integer) (`Failed?` :type Boolean))
  (bind _amountremaining (`local.AmountRemaining`))
  (bind _item_info (`local.Item Info`))
  (bind _item_info_2 (`local.Item Info`))
  (set `local.AmountRemaining` `Item Amount`)
  (while (and (> (`local.AmountRemaining`) 0) (not (`local.Failed?`)))
    (bind (_index _found_) (`self.FindSlot` (`local.Item Name`)))
    (if _found_
      (if (not (< (`local.AmountRemaining`) 1))
        (`self.IncreaseStack` _index 0 _item_info)
        (bind _result (`/Engine/EditorBlueprintResources/StandardMacros.DecrementInt` (`local.AmountRemaining`))
          (:`  `
            (return true _result)))
        (else
          (`self.IncreaseStack` _index 0 _item_info)
          (bind _output_get (set `local.AmountRemaining` (- (`local.AmountRemaining`) (`local.AmountRemaining`))))
          (return true _output_get)))
      (elif (`self.SlotsAvailable`)
        (if (not (< _amountremaining 1))
          (bind _created (`self.CreateStack` (`local.Item Name`) 0 _item_info_2))
          (if _created
            (bind _result_2 (`/Engine/EditorBlueprintResources/StandardMacros.DecrementInt` (`local.AmountRemaining`))
              (:`  `
                (return true _result_2))))
          (else
            (bind _created_2 (`self.CreateStack` (`local.Item Name`) _amountremaining _item_info_2))
            (if _created_2
              (bind _output_get_2 (set `local.AmountRemaining` (- (`local.AmountRemaining`) (`local.AmountRemaining`))))
              (return true _output_get_2))))
        (else
          (return false 0)))))
  (return false 0))

(fn `AddToInventory`
  (params (ItemID :type Name) (Quantity :type Integer))
  (returns (Success :type Boolean) (QuantityRemaining :type Integer))
  (locals (Local_QuantityRemaining :type Integer) (Local_HasFailed :type Boolean))
  (set `local.Local_QuantityRemaining` Quantity)
  (while (and (> (`local.Local_QuantityRemaining`) 0) (not (`local.Local_HasFailed`)))
    (bind (_index _found_) (`self.FindSlot` (`local.ItemID`)))
    (if _found_
      (`self.IncreaseStack` _index 1)
      (`/Engine/EditorBlueprintResources/StandardMacros.DecrementInt` (`local.Local_QuantityRemaining`))
      (elif (`self.SlotsAvailable`)
        (bind _created (`self.CreateStack` (`local.ItemID`) 1))
        (if _created
          (`/Engine/EditorBlueprintResources/StandardMacros.DecrementInt` (`local.Local_QuantityRemaining`))
          (else
            (set `local.Local_HasFailed` true)))
        (else
          (set `local.Local_HasFailed` true)))))
  (return (not (`local.Local_HasFailed`)) (`local.Local_QuantityRemaining`)))

(fn `ChangeSlot`
  (params (`Item Name` :type Name) (`Item Amount` :type "Float (double-precision)")))

(fn `CreateStack`
  (params (Item :type Name) (Amount :type Integer) (`Item Info` :type "/Game/HUD/Structs/Struct_ItemInfo Structure"))
  (returns (Created :type Boolean))
  (bind (_name _description _itemclass _icon _mesh _stackable _itemamount _stacklimit _durability _maxdurability _weight _value) (break `/Game/HUD/Structs/Struct_ItemInfo` `Item Info`))
  (bind (_emptyslot _indexavailable) (`self.SlotsAvailable`))
  (if _emptyslot
    (`KismetArrayLibrary.Array_Set` (`self.Contents`) _indexavailable (make `/Game/HUD/Structs/Struct_ItemInfo` (`local.Item`) _description _itemclass _icon _mesh _stackable (`local.Amount`) 0 _durability _maxdurability _weight _value))
    (return true)
    (else
      (return false))))

(fn `DEBUG_PrintContents`
  (for (_array_element _array_index) (`self.Contents`)
    (bind (_name _description _itemclass _icon _mesh _stackable _itemamount) (break `/Game/HUD/Structs/Struct_ItemInfo` _array_element))
    (`KismetSystemLibrary.PrintString` (`KismetStringLibrary.Concat_StrStr` (`KismetStringLibrary.Conv_IntToString` _array_index) ":" (`KismetStringLibrary.Conv_NameToString` _name) "=" (`KismetStringLibrary.Conv_IntToString` _itemamount)))))

(fn `FindSlot`
  (params (ItemID :type Name))
  (returns (Index :type Integer) (`Found?` :type Boolean))
  (for (_array_element _array_index) (`self.Contents`)
    (if (== (`.Name_2_E2CF82EC45EEAE137E073BAAFD686EB9` (break `/Game/HUD/Structs/Struct_ItemInfo` _array_element)) (`local.ItemID`))
      (if (< (`self.GetStackSize` (`local.ItemID`)) 0)
        (return _array_index true))))
  (return -1 false))

(fn `GetStackSize`
  (params (ItemID :type Name))
  (returns (StackLimit :type Integer))
  (bind _returnvalue (`|GetDataTableRow` "/Game/Items/DataTables/DT_Items.DT_Items" ItemID)
    (:`then`
      (return (`.StackLimit_35_EB2A4E0E409D2C455D61FEA2E3E6EE81` (break `/Game/HUD/Structs/Struct_ItemInfo` _returnvalue))))
    (:`RowNotFound`
      (return 0))))

(fn `IncreaseStack`
  (params (Index :type Integer) (Amount :type Integer) (`Item Info` :type "/Game/HUD/Structs/Struct_ItemInfo Structure"))
  (bind _contents (`self.Contents`))
  (bind (_output_name _output_description _output_itemclass _output_icon _output_mesh _output_stackable _output_itemamount _output_stacklimit _output_durability _output_maxdurability _output_weight _output_value) (break `/Game/HUD/Structs/Struct_ItemInfo` (`|GetArrayItem` _contents Index)))
  (`KismetArrayLibrary.Array_Set` _contents Index (make `/Game/HUD/Structs/Struct_ItemInfo` _output_name _output_description _output_itemclass _output_icon _output_mesh _output_stackable (+ _output_itemamount Amount) _output_stacklimit _output_durability _output_maxdurability _output_weight _output_value)))

(fn `Remove`)

(fn `SlotsAvailable`
  (returns (EmptySlot :type Boolean) (IndexAvailable :type Integer))
  (for (_array_element _array_index) (`self.Contents`)
    (bind (_name _description _itemclass _icon _mesh _stackable _itemamount) (break `/Game/HUD/Structs/Struct_ItemInfo` _array_element))
    (if (and (== _name "None") (== _itemamount 0))
      (return true _array_index)))
  (return false -1))