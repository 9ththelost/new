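; AC_ItemInfo is an item data component that gives its owning actor an item ID, data table info and quantity.
; On BeginPlay it turns on owner replication, looks up the item's data table row, caches it and sets quantity to one.
; Interact is empty and Looking returns placeholder text.
; The logic that adds the item to an inventory component and destroys the owner is disconnected and never runs.
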(event `self.ReceiveBeginPlay`
  (bind (_itemid_datatable _itemid_rowname) (break `DataTableRowHandle` (`self.ItemID`)))
  (`|ExecutionSequence`
    (:`then_0`
      (`Actor.SetReplicates` (`self.GetOwner`) true))
    (:`then_1`
      (if true
        (bind _returnvalue (`|GetDataTableRow` _itemid_datatable _itemid_rowname)
          (:`then`
            (set `self.CurrentInfo` _returnvalue)
            (set `self.Quantity` 1)))))))

(event `/Game/HUD/Blueprints/I_Interacting.Interact`
  (params (PlayerCharacter :type "/Game/Characters/Player/BP_ThirdPersonCharacter Object Reference")))

(fn `Looking`
  (params (`Looking Player` :type "/Game/Characters/Player/BP_ThirdPersonCharacter Object Reference"))
  (returns (`Object Name` :type Name) (`Object Info` :type Text))
  (return "None" ""))