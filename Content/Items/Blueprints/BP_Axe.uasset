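; BP_Axe is an axe item whose stats depend on its material tier: Wood, Stone or Iron.
; On BeginPlay it calls GetType, which switches on Material to set max durability, tool damage and attack damage, starting Durability at full.
; Stats rise with each tier, while all three tiers assign the same test mesh.
; A GetCurrent event exposes material, durability and damage parameters but has no logic.
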(event `self.ReceiveBeginPlay`
  (`self.GetType` (`self.Material`)))

(event `GetType`
  (params (Material :type "/Game/Items/Enumerators/E_ItemMaterial Enum" :default "NewEnumerator0"))
  (switch `/Game/Items/Enumerators/E_ItemMaterial` Material
    (:`NewEnumerator0`
      (bind _output_get (set `self.MaxDurability` 100.0))
      (set `self.Durability` _output_get)
      (set `self.ToolDamage` 2.0)
      (set `self.AttackDamage` 8.0)
      (set `self.StaticMesh` "/Game/Items/StaticMeshs/SM_TestAxe.SM_TestAxe"))
    (:`NewEnumerator1`
      (bind _output_get_2 (set `self.MaxDurability` 300.0))
      (set `self.Durability` _output_get_2)
      (set `self.ToolDamage` 5.0)
      (set `self.AttackDamage` 15.0)
      (set `self.StaticMesh` "/Game/Items/StaticMeshs/SM_TestAxe.SM_TestAxe"))
    (:`NewEnumerator2`
      (bind _output_get_3 (set `self.MaxDurability` 500.0))
      (set `self.Durability` _output_get_3)
      (set `self.ToolDamage` 8.0)
      (set `self.AttackDamage` 25.0)
      (set `self.StaticMesh` "/Game/Items/StaticMeshs/SM_TestAxe.SM_TestAxe")))
  (set `self.Material` Material))

(event `GetCurrent`
  (params (Material :type "/Game/Items/Enumerators/E_ItemMaterial Enum" :default "NewEnumerator0") (Durability :type "Float (double-precision)") (`Tool Damage` :type "Float (double-precision)") (`Attack Damage` :type "Float (double-precision)")))

(fn `UserConstructionScript`)